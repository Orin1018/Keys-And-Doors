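; BP_fallingplatform is a platform that falls after the third-person character steps on it, then returns to its starting place.
; A box overlap triggers it, and a delay precedes switching on physics simulation to drop the mesh.
; After a falling delay, physics switches off and a timeline lerps the transform back to the one saved at BeginPlay.
; A ready flag blocks retriggering until the return finishes, with debug prints throughout.
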(event OnComponentBeginOverlap(Box)
  (params (OverlappedComponent :type Primitive%20Component%20Object%20Reference) (OtherActor :type Actor%20Object%20Reference) (OtherComp :type Primitive%20Component%20Object%20Reference) (OtherBodyIndex :type Integer) (bFromSweep :type Boolean) (SweepResult :type Hit%20Result%20Structure%20%28by%20ref%29))
  (Development|PrintString "Somemthing is standing on me")
  (Utilities|Casting|CastToBP_ThirdPersonCharacter OtherActor)
  (if (Variables|Default|GetIsReady)
    (CallFunction|Activate)
    (Variables|Default|SetIsReady false)
    (else
      (Development|PrintString "Cooling Down"))))

(event Custom|Activate
  (Development|PrintString "activated")
  (Utilities|FlowControl|Delay (Variables|PlatformSettings|GetFall%20Delay%20Duration))
  (CallFunction|Falling))

(event Custom|Falling
  (Development|PrintString "falling")
  (Physics|SetSimulatePhysics (Variables|Default|GetPlatform_0) true)
  (Utilities|FlowControl|Delay (Variables|PlatformSettings|GetFalling%20Duration))
  (CallFunction|Reset))

(event Custom|Reset
  (Development|PrintString "Resetting the platform")
  (Physics|SetSimulatePhysics (Variables|Default|GetPlatform_0) false)
  (Variables|Default|SetFallen%20Transform (Transformation|GetWorldTransform (Variables|Default|GetPlatform_0)))
  (bind _lerp (Timeline|GoBacktoStartTransform PlayFromStart)
    (:Update
      (Transformation|SetWorldTransform (Variables|Default|GetPlatform_0) (Math|Transform|Lerp(Transform) (Variables|Default|GetFallen%20Transform) (Variables|Default|GetStarting%20Transform) _lerp) false false))
    (:Finished
      (Variables|Default|SetIsReady true))))

(event EventBeginPlay
  (Variables|Default|SetStarting%20Transform (Transformation|GetWorldTransform (Variables|Default|GetPlatform_0)))
  (Variables|Default|SetIsReady true))

(fn ConstructionScript)