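; BP_manager is a wave manager actor that coordinates enemy spawners and drops a key when a wave is nearly or fully cleared.
; NewEnemyWaveCheck counts BP_Enemy actors and, when one or none remain, spawns a BP_Key at the passed transform after a short delay.
; SpawnNewEnemy waits, then calls SpawnNewEnemy on every BP_enemyspawner in the level.
; Debug prints report manager startup, spawner count and wave progress.
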(event Custom|NewEnemyWaveCheck
  (params (SpawnTransform :type Transform))
  (Development|PrintString "Checking enemy count")
  (bind _outactors (Actor|GetAllActorsOfClass "/Game/Blueprints/BP_Enemy.BP_Enemy_C"))
  (if (> (Utilities|Array|Length _outactors) 1)
    (Development|PrintString "There are still more enemies")
    (else
      (Utilities|FlowControl|Delay 3.0)
      (Game|SpawnActorfromClass "/Game/Blueprints/BP_Key.BP_Key_C" SpawnTransform "Undefined" "MultiplyWithRoot" 0 0))))

(event Custom|SpawnNewEnemy
  (Development|PrintString "Spawning new enemies in 4 seconds")
  (Utilities|FlowControl|Delay 4.0)
  (bind _outactors (Actor|GetAllActorsOfClass "/Game/Blueprints/BP_enemyspawner.BP_enemyspawner_C"))
  (for (_array_element _array_index) _outactors
    (Default|SpawnNewEnemy _array_element)
    (Development|PrintString "Hello" true true (Utilities|Struct|MakeLinearColor (Math|Random|RandomFloat) (Math|Random|RandomFloat) (Math|Random|RandomFloat) 0.0)))
  (Development|PrintString "New Wave Completed"))

(event EventBeginPlay
  (Development|PrintString "spawn manager is active")
  (bind _outactors (Actor|GetAllActorsOfClass "/Game/Blueprints/BP_enemyspawner.BP_enemyspawner_C"))
  (Development|PrintString (Utilities|String|Append "There are " (Utilities|String|ToString(Integer) (Utilities|Array|Length _outactors)) " spawners in the level " "there are " "## " "enemies in the level ")))

(fn ConstructionScript)